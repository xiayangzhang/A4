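; Enemy character Blueprint for an AI-controlled gunner that runs a behavior tree and fights with a child-actor gun.
; On possession and every Tick, it copies health and perception state to the blackboard and updates its out-of-ammo flag.
; At low health it clears its room's enemy flag and destroys itself and its controller.
; Fire adds random spread and turns the body, while Reload plays a montage, waits its length, then refills the gun.
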(event `self.ReceiveBeginPlay`
  (set `self.PerceptionComponent` (`self.AIPerception`))
  (set `self.HearComponent` (`self.HearPerception`)))

(event `self.ReceivePossessed`
  (params (NewController :type "Controller Object Reference"))
  (bind _returnvalue (`AIBlueprintHelperLibrary.GetAIController` NewController))
  (`AIController.RunBehaviorTree` _returnvalue "/Game/Blueprints/BT/EnemyBT.EnemyBT")
  (bind _blackboardcomponent (`AIController.UseBlackboard` _returnvalue "/Game/Blueprints/BT/EnemyBB.EnemyBB"))
  (`/Engine/EditorBlueprintResources/StandardMacros.IsValid` null :!label _label
    (:`Is Valid`
      _)
    (:`Is Not Valid`
      _))
  (bind _returnvalue_2 (`HealthComponent.HealthPercentageRemaining` (`self.Health`)))
  (`BlackboardComponent.SetValueAsFloat` _blackboardcomponent (`self.HealthRemainingBB`) _returnvalue_2)
  (`BlackboardComponent.SetValueAsBool` _blackboardcomponent (`self.CanSee`) (`self.bCanSeeActor`))
  (`BlackboardComponent.SetValueAsBool` _blackboardcomponent (`self.Noticed`) (`self.bNoticedActor`))
  (`BlackboardComponent.SetValueAsObject` _blackboardcomponent (`self.player`) (`self.DetectedActor`))
  (bind _asgun_blueprint (cast `/Game/Blueprints/GunBlueprint` (`ChildActorComponent.ChildActor` (`self.Gun`))))
  (if (<= (`/Game/Blueprints/GunBlueprint.RoundsRemainingInMagazine` _asgun_blueprint) 0)
    (set `self.bOutOfAmmo` true)
    (else
      (set `self.bOutOfAmmo` false)))
  (if (< (`HealthComponent.CurrentHealth` (`self.Health`)) 5.0)
    (bind _asroom_bp (cast `/Game/Blueprints/RoomBP` (`self.RoomBelong`)))
    (if true
      (set `Room.HasEnemy` false _asroom_bp)
      (`self.K2_DestroyActor` (`AIBlueprintHelperLibrary.GetAIController` self))
      (`self.K2_DestroyActor`))))

(event `self.ReceiveTick`
  (params (DeltaSeconds :type "Float (single-precision)"))
  (goto _label))

(event `self.Fire`
  (params (FireDirection :type "Vector Structure"))
  (bind _asgun_blueprint (cast `/Game/Blueprints/GunBlueprint` (`ChildActorComponent.ChildActor` (`self.Gun`))))
  (`/Game/Blueprints/GunBlueprint.Fire` _asgun_blueprint (+ (* (`KismetMathLibrary.RandomUnitVector`) (`self.TargetAccuracyOffset`)) FireDirection))
  (`self.K2_SetActorRotation` (`KismetMathLibrary.Conv_VectorToRotator` FireDirection)))

(event `self.Reload`
  (bind _reloadanimationlength (`self.ReloadStart`))
  (`KismetSystemLibrary.Delay` _reloadanimationlength)
  (`self.ReloadEnd`))

(fn `New Walk Speed`
  (params (speed :type "Float (double-precision)"))
  (set `CharacterMovementComponent.MaxWalkSpeed` 0.0 (`self.CharacterMovement`)))

(fn `ReloadEnd`
  (bind _asgun_blueprint (cast `/Game/Blueprints/GunBlueprint` (`ChildActorComponent.ChildActor` (`self.Gun`))))
  (set `self.bIsReloading` false)
  (set `self.bOutOfAmmo` false)
  (`/Game/Blueprints/GunBlueprint.Reload` _asgun_blueprint))

(fn `ReloadStart`
  (returns (ReloadAnimationLength :type "Float (double-precision)"))
  (bind _returnvalue (`AnimInstance.Montage_Play` (`SkeletalMeshComponent.GetAnimInstance` (`self.Mesh`)) "/Game/Assets/Mannequin/AnimStarterPack/ReloadRifleHip_Montage.ReloadRifleHip_Montage" 1.0 "MontageLength" 0.0 true))
  (bind _asgun_blueprint (cast `/Game/Blueprints/GunBlueprint` (`ChildActorComponent.ChildActor` (`self.Gun`))))
  (set `/Game/Blueprints/GunBlueprint.RoundsRemainingInMagazine` 0 _asgun_blueprint)
  (set `/Game/Blueprints/GunBlueprint.bCanFire` false _asgun_blueprint)
  (set `self.bIsReloading` true)
  (return _returnvalue))

(fn `UserConstructionScript`)