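; PK_BP is a point pickup that the player collects by overlapping its Box.
; Overlap calls Newaddpoint on the PlayerCharacterBlueprint, destroys the pickup, and pauses the game when Totalpoint equals 15.
; Otherwise it casts the same overlapping actor to Room to spawn a replacement at GenRandomPos, a cast that fails unless the player class derives from Room.
; A local Addpoint function increments Point but is not called here.
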(event `self.Box.OnComponentBeginOverlap`
  (params (OverlappedComponent :type "PrimitiveComponent Object Reference") (OtherActor :type "Actor Object Reference") (OtherComp :type "PrimitiveComponent Object Reference") (OtherBodyIndex :type Integer) (bFromSweep :type Boolean) (SweepResult :type "HitResult Structure (by ref)"))
  (bind _asplayer_character_blueprint (cast `/Game/Blueprints/PlayerCharacterBlueprint` OtherActor))
  (`/Game/Blueprints/PlayerCharacterBlueprint.newaddpoint` _asplayer_character_blueprint)
  (`self.K2_DestroyActor`)
  (if (== 15 (`/Game/Blueprints/PlayerCharacterBlueprint.totalpoint` _asplayer_character_blueprint))
    (`GameplayStatics.SetGamePaused` true)
    (else
      (bind _asroom (cast `Room` OtherActor))
      (bind _returnvalue (`Room.GenRandomPos` _asroom))
      (`|SpawnActorFromClass` "PK_BP_C" (`KismetMathLibrary.Conv_VectorToTransform` _returnvalue) "Undefined" "OverrideRootScale" null null))))

(fn `addpoint`
  (set `self.point` (+ (`self.point`) 1)))

(fn `UserConstructionScript`)