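; RoomBP is a room Blueprint that triggers enemy generation and detects the player entering through a box collision.
; Its Init event calls GenEnemy, then sizes the box to half the room's width and length with a fixed vertical extent.
; When an actor of exactly the PlayerCharacterBlueprint class begins overlapping the box and HasEnemy is false, it calls GenEnemy again.
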(event `self.init`
  (`self.GenEnemy`)
  (`BoxComponent.SetBoxExtent` (`self.collision`) (`KismetMathLibrary.MakeVector` (/ (`self.RoomWidth`) 2.0) (/ (`self.RoomLength`) 2.0) 400.0) true))

(event `self.collision.OnComponentBeginOverlap`
  (params (OverlappedComponent :type "PrimitiveComponent Object Reference") (OtherActor :type "Actor Object Reference") (OtherComp :type "PrimitiveComponent Object Reference") (OtherBodyIndex :type Integer) (bFromSweep :type Boolean) (SweepResult :type "HitResult Structure (by ref)"))
  (if (== (`GameplayStatics.GetObjectClass` OtherActor) "/Game/Blueprints/PlayerCharacterBlueprint.PlayerCharacterBlueprint_C")
    (if (== (`self.HasEnemy`) false)
      (`self.GenEnemy`))))

(fn `UserConstructionScript`)