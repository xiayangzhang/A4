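; BP_GoodParticleProjectile is a particle-based projectile actor that bursts into an explosion effect on overlap.
; The construction script assigns the main particle template to its MainParticle component.
; On overlap with any actor other than its instigator, it deactivates that particle and spawns the explosion emitter at its location, without applying damage or destroying itself.
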(event `self.ReceiveBeginPlay`)

(event `self.ReceiveActorBeginOverlap`
  (params (OtherActor :type "Actor Object Reference"))
  ;[1 1 1] Ignore Owner Collision
  (if (not (== OtherActor (`self.GetInstigator`)))
    (`ActorComponent.Deactivate` (`self.Main Particle`))
    ;[1 1 1] Spawn Explosion Particle
    (`GameplayStatics.SpawnEmitterAtLocation` (`self.GoodParticleProjectile Explosion`) (`self.K2_GetActorLocation`))))

(fn `UserConstructionScript`
  (`ParticleSystemComponent.SetTemplate` (`self.Main Particle`) (`self.GoodParticleProjectile Main`)))