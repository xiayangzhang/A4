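; BP_GoodParticleProjectile_Showcase is a demo actor that shows a looping projectile particle effect with its explosion.
; The construction script assigns the main projectile template to its particle component.
; On overlap it deactivates that particle, spawns the explosion emitter at the actor's location, then reactivates the main particle after a short delay so the showcase can repeat.
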(event `self.ReceiveBeginPlay`)

(event `self.ReceiveActorBeginOverlap`
  (params (OtherActor :type "Actor Object Reference"))
  (bind _main_particle (`self.Main Particle`))
  (`ActorComponent.Deactivate` _main_particle)
  ;[1 1 1] Spawn Explosion Particle
  (`GameplayStatics.SpawnEmitterAtLocation` (`self.GoodParticleProjectile Explosion`) (`self.K2_GetActorLocation`))
  ;[1 1 1] For Loop
  (`KismetSystemLibrary.Delay` 0.8)
  (`ActorComponent.Activate` _main_particle false))

(fn `UserConstructionScript`
  (`ParticleSystemComponent.SetTemplate` (`self.Main Particle`) (`self.GoodParticleProjectile Main`)))